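; Trigger box actor that fires a one-shot sound and door close, apparently for the first bedside dialog.
; Begin and end overlap on the Triggerbox set a flag, which Tick polls.
; A used flag and a DoOnce limit it to one firing, which plays a sound cue at the actor's location.
; It then casts its owner to DoorBP, closes that door and marks it ready.
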(event `self.ReceiveTick`
  (params (DeltaSeconds :type "Float (single-precision)"))
  (if (`self.onOverlap`)
    (if (not (`self.Used_04`))
      (set `self.Used_04` true)
      (`/Engine/EditorBlueprintResources/StandardMacros.DoOnce` false
        (:`Completed`
          (`GameplayStatics.PlaySoundAtLocation` "/Game/Audio/Dialog/03_SC.03_SC" (`self.K2_GetActorLocation`))
          (bind _asdoor_bp (cast `/Game/Door/DoorBP` (`self.GetOwner`)))
          (`/Game/Door/DoorBP.Close_Door` _asdoor_bp)
          (set `/Game/Door/DoorBP.DoorReady` true _asdoor_bp))))))

(event `self.Triggerbox.OnComponentBeginOverlap`
  (params (OverlappedComponent :type "PrimitiveComponent Object Reference") (OtherActor :type "Actor Object Reference") (OtherComp :type "PrimitiveComponent Object Reference") (OtherBodyIndex :type Integer) (bFromSweep :type Boolean) (SweepResult :type "HitResult Structure (by ref)"))
  (set `self.onOverlap` true))

(event `self.Triggerbox.OnComponentEndOverlap`
  (params (OverlappedComponent :type "PrimitiveComponent Object Reference") (OtherActor :type "Actor Object Reference") (OtherComp :type "PrimitiveComponent Object Reference") (OtherBodyIndex :type Integer))
  (set `self.onOverlap` false))

(fn `UserConstructionScript`)