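; A grabbable book prop that the player picks up and drops with a motion controller.
; Pickup turns off mesh physics, attaches the root to the supplied component keeping world transform, and plays a book sound at the actor's location.
; Drop re-enables physics and detaches the book in place.
; The sound sits behind a DoOnce inside a function, whose state does not persist between calls.
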(event `/Game/VirtualRealityBP/Blueprints/PickupActorInterface.Pickup`
  (params (AttachTo :type "SceneComponent Object Reference"))
  (`PrimitiveComponent.SetSimulatePhysics` (`self.StaticMeshComponent`) false)
  (`SceneComponent.K2_AttachToComponent` (`self.K2_GetRootComponent`) AttachTo "None" "KeepWorld" "KeepWorld" "KeepWorld" false)
  (`self.PlayInteractionSound`))

(event `/Game/VirtualRealityBP/Blueprints/PickupActorInterface.Drop`
  (`PrimitiveComponent.SetSimulatePhysics` (`self.StaticMeshComponent`) true)
  (`self.K2_DetachFromActor` "KeepWorld" "KeepWorld" "KeepWorld"))

(fn `PlayInteractionSound`
  (`/Engine/EditorBlueprintResources/StandardMacros.DoOnce` false
    (:`Completed`
      (`GameplayStatics.PlaySoundAtLocation` "/Game/Audio/Book_SC.Book_SC" (`self.K2_GetActorLocation`)))))

(fn `UserConstructionScript`)