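; VR door Blueprint that swings open with a sound when either grab input is pressed while something overlaps its Box.
; Box overlap events set the flag checked by the grab inputs, and IsOpen guards the snap rotation in OpenDoor and CloseDoor.
; Functions not called here close the door, teleport the MotionControllerPawn with camera fades, and, when DoorReady, play a sound and reveal a CharacterUB_BP mesh.
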(event `InputAction|GrabLeft` :consume false
  (params (Key :type "Key Structure" :default "AnyKey"))
  (:`Pressed`
    (if (`self.isOverlapped`) :!label _label
      (`self.Open_Door`))))

(event `self.ReceiveBeginPlay`
  (`self.EnableInput` (`GameplayStatics.GetPlayerController` 0)))

(event `InputAction|GrabRight` :consume false
  (params (Key :type "Key Structure" :default "AnyKey"))
  (:`Pressed`
    (goto _label)))

(event `self.Box.OnComponentBeginOverlap`
  (params (OverlappedComponent :type "PrimitiveComponent Object Reference") (OtherActor :type "Actor Object Reference") (OtherComp :type "PrimitiveComponent Object Reference") (OtherBodyIndex :type Integer) (bFromSweep :type Boolean) (SweepResult :type "HitResult Structure (by ref)"))
  (set `self.isOverlapped` true))

(event `self.Box.OnComponentEndOverlap`
  (params (OverlappedComponent :type "PrimitiveComponent Object Reference") (OtherActor :type "Actor Object Reference") (OtherComp :type "PrimitiveComponent Object Reference") (OtherBodyIndex :type Integer))
  (set `self.isOverlapped` false))

(fn `Close_Door`
  (if (`self.isOpen`)
    (`/Engine/EditorBlueprintResources/StandardMacros.DoOnce` false
      (:`Completed`
        (`GameplayStatics.PlaySoundAtLocation` "/Game/Audio/Door_Closing.Door_Closing" (`self.K2_GetActorLocation` (`ActorComponent.GetOwner` (`self.SM_Door`))))
        (`SceneComponent.K2_SetWorldRotation` (`self.SM_Door`) (struct) false false)
        (set `self.isOpen` false)))))

(fn `Fade&Translate`
  (bind _returnvalue (`GameplayStatics.GetPlayerCameraManager` 0))
  (bind _asmotion_controller_pawn (cast `/Game/VirtualRealityBP/Blueprints/MotionControllerPawn` (`GameplayStatics.GetPlayerPawn` 0)))
  (`self.K2_TeleportTo` :`self` _asmotion_controller_pawn :`DestLocation` (0.1 0.0 0.0))
  (`PlayerCameraManager.StartCameraFade` :`self` _returnvalue :`FromAlpha` 1.0 :`Duration` 0.2)
  (`PlayerCameraManager.StartCameraFade` :`self` _returnvalue :`ToAlpha` 1.0 :`Duration` 0.2))

(fn `LookAtDoor`
  (if (`self.DoorReady`)
    (`/Engine/EditorBlueprintResources/StandardMacros.DoOnce` false
      (:`Completed`
        (`GameplayStatics.PlaySoundAtLocation` "/Game/Audio/Dialog/15_SC.15_SC" (`self.K2_GetActorLocation`))
        (bind _outactors (`GameplayStatics.GetAllActorsOfClass` "/Game/Characters/GirlReg/CharacterUB_BP.CharacterUB_BP_C"))
        (`SceneComponent.SetVisibility` (`Character.Mesh` (cast `/Game/Characters/GirlReg/CharacterUB_BP` (`KismetArrayLibrary.Array_Get` _outactors) :!pure true)) true true)))))

(fn `Open_Door`
  (if (not (`self.isOpen`))
    (`/Engine/EditorBlueprintResources/StandardMacros.DoOnce` false
      (:`Completed`
        (`GameplayStatics.PlaySoundAtLocation` "/Game/Audio/Door_Opening.Door_Opening" (`self.K2_GetActorLocation` (`ActorComponent.GetOwner` (`self.SM_Door`))))
        (`SceneComponent.K2_SetWorldRotation` (`self.SM_Door`) (struct :`Yaw` 90.0) false false)
        (set `self.isOpen` true)))))

(fn `UserConstructionScript`)